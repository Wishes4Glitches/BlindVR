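; Throwable-style VR ball interactable that a motion controller can pick up and drop, and that knocks NPCs into physics simulation on contact.
; Pickup, called by BP_MotionController, disables the mesh's physics and attaches the actor to the given component, keeping its world transform.
; Drop re-enables physics and detaches it.
; Any mesh hit on an NPC turns on physics for that NPC's mesh, with no check on impact speed or held state.
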(event `/Game/Blueprints/Player/PickupActorInterface.Pickup`
  (params (AttachTo :type "SceneComponent Object Reference"))
  (`PrimitiveComponent.SetSimulatePhysics` (`self.StaticMeshComponent`) false)
  (`SceneComponent.K2_AttachToComponent` (`self.K2_GetRootComponent`) AttachTo "None" "KeepWorld" "KeepWorld" "KeepWorld" false))

(event `/Game/Blueprints/Player/PickupActorInterface.Drop`
  (`PrimitiveComponent.SetSimulatePhysics` (`self.StaticMeshComponent`) true)
  (`self.K2_DetachFromActor` "KeepWorld" "KeepWorld" "KeepWorld"))

(event `self.StaticMeshComponent.OnComponentHit`
  (params (HitComponent :type "PrimitiveComponent Object Reference") (OtherActor :type "Actor Object Reference") (OtherComp :type "PrimitiveComponent Object Reference") (NormalImpulse :type "Vector Structure") (Hit :type "HitResult Structure (by ref)"))
  (bind _asnpc (cast `/Game/AI/NPC/NPC` OtherActor))
  (`PrimitiveComponent.SetSimulatePhysics` (`Character.Mesh` _asnpc) true))

(fn `UserConstructionScript`)